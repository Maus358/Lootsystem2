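; BP_StoringStats is a helper Blueprint that picks and increases stat entries, each holding a name and a value.
; RandomSelection returns a random array element using a fixed index range that assumes at least five entries.
; UpdatingValue adds a fixed amount to a stat through a by-ref set, keeps its name, and prints the value.
; The event graph and construction script are empty, and neither function is called within the Blueprint.
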(fn `Random Selection`
  (params (Array :type "Array of /Game/Blueprints/Structs/S_Stats Structure"))
  (returns (`Selected Stat` :type "/Game/Blueprints/Structs/S_Stats Structure (by ref)"))
  (return (`|GetArrayItem` Array (`KismetMathLibrary.RandomIntegerInRange` 0 4))))

(fn `UpdatingValue`
  (params (SelectedStat :type "/Game/Blueprints/Structs/S_Stats Structure"))
  (bind (_name _value) (break `/Game/Blueprints/Structs/S_Stats` SelectedStat))
  (`|VariableSetRef` SelectedStat (make `/Game/Blueprints/Structs/S_Stats` _name (+ _value 10.0)))
  (`KismetSystemLibrary.PrintString` (`KismetStringLibrary.Conv_DoubleToString` (`.Value_5_4680C3C849685626042282A5900F5AF8` (break `/Game/Blueprints/Structs/S_Stats` SelectedStat))))
  (return))

(fn `UserConstructionScript`)